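; PC_Mym is a player controller that handles the player's sessions at a vending machine POS.
; Beginning use teleports the character to the machine's target transform at its current height, aligns control rotation, and creates the POS widget if none is cached, passing it the shopper and machine.
; It then shows the widget with UI-only input and a cursor.
; Ending use restores game input, hides the cursor and removes the widget without clearing its reference.
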(event `BeginUsingPOSMachine`
  (params (`Pos Machine` :type "/Game/_Game/Props/Machine/BP_POS_Machine Object Reference"))
  (bind _returnvalue (`self.GetMymCharacter`))
  (bind _playertargettransform (`/Game/_Game/Props/Machine/BP_POS_Machine.PlayerTargetTransform` `Pos Machine`))
  (bind (_returnvalue_x _returnvalue_y _returnvalue_z) (`KismetMathLibrary.BreakVector` (`self.K2_GetActorLocation` _returnvalue)))
  (bind (_returnvalue_x_2 _returnvalue_y_2) (`KismetMathLibrary.BreakVector` (`SceneComponent.K2_GetComponentLocation` _playertargettransform)))
  (`self.K2_SetActorLocation` _returnvalue (`KismetMathLibrary.MakeVector` _returnvalue_x_2 _returnvalue_y_2 _returnvalue_z) false true)
  (`self.SetControlRotation` self (`SceneComponent.K2_GetComponentRotation` _playertargettransform))
  (if (not (`KismetSystemLibrary.IsValid` (`self.Pos Widget`)))
    (bind _returnvalue_2 (`|CreateWidget` "/Game/_Game/Widgets/WBP_VendingMachine_POS.WBP_VendingMachine_POS_C" self))
    (`/Game/_Game/Widgets/WBP_VendingMachine_POS.ConstructVendingMachine` _returnvalue_2 (`MymCharacter.GetShopper` (`self.GetMymCharacter`)) self `Pos Machine`)
    (set `self.Pos Widget` _returnvalue_2))
  (`UserWidget.AddToPlayerScreen` _returnvalue_2 0)
  (`WidgetBlueprintLibrary.SetInputMode_UIOnlyEx` self _returnvalue_2)
  (set `self.bShowMouseCursor` true))

(event `EndUsingPOSMachine`
  (`WidgetBlueprintLibrary.SetInputMode_GameOnly` self)
  (set `self.bShowMouseCursor` false)
  (`Widget.RemoveFromParent` (`self.Pos Widget`)))

(fn `UserConstructionScript`)
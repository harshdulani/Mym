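; BP_CarpenterMachine is an actor for a carpenter machine with three numbered buttons and a Done button, currently implementing only their press animation.
; A PressButton event takes a button mesh and plays the ButtonClick timeline to offset its relative location along local Y.
; Four debug keys trigger the presses.
; All buttons share one timeline instance, so overlapping presses break each other's animation.
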(event Custom|PressButton
  (params (Mesh :type Static%20Mesh%20Component%20Object%20Reference))
  ;[0.15 0.15 0.15 0.5] this is a single instance, so it will break animations for other buttons if called in the middle of another button's anim
  (bind _localy (Timeline|ButtonClick PlayFromStart)
    (:Update
      (Transformation|SetRelativeLocation Mesh (Math|Vector|MakeVector 0.0 (* _localy -5.0) 0.0) false false))))

(event EventBeginPlay)

(event Collision|EventActorBeginOverlap
  (params (OtherActor :type Actor%20Object%20Reference)))

(event EventTick
  (params (DeltaSeconds :type Float%20%28single-precision%29)))

(event Input|KeyboardEvents|DebugKey1
  (params (Key :type Key%20Structure :default "None") (ActionValue :type Input%20Action%20Value%20Structure))
  (:Pressed
    (CallFunction|PressButton (Variables|Default|GetButtonMesh1))))

(event Input|KeyboardEvents|DebugKey2
  (params (Key :type Key%20Structure :default "None") (ActionValue :type Input%20Action%20Value%20Structure))
  (:Pressed
    (CallFunction|PressButton (Variables|Default|GetButtonMesh2))))

(event Input|KeyboardEvents|DebugKey3
  (params (Key :type Key%20Structure :default "None") (ActionValue :type Input%20Action%20Value%20Structure))
  (:Pressed
    (CallFunction|PressButton (Variables|Default|GetButtonMesh3))))

(event Input|KeyboardEvents|DebugKey4
  (params (Key :type Key%20Structure :default "None") (ActionValue :type Input%20Action%20Value%20Structure))
  (:Pressed
    (CallFunction|PressButton (Variables|Default|GetButtonMeshDone))))

(fn ConstructionScript)
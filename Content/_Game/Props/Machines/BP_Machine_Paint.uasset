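; BP_Machine_Paint is a paint machine prop with three numbered buttons and a Done button.
; Each interaction's begin event only calls PressButtonAnim with a button mesh, an interaction component and the interacting tracker.
; Buttons 1 and 2 are cross-wired: each event passes the other's mesh and interaction.
; Resource spawn point and player controller lookups are unconnected, so no painting or spawning happens in this graph.
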(event `self.Interaction2.OnInteractBegin`
  (params (ByTracker :type "InteractionTrackerComponent Object Reference"))
  (`self.PressButtonAnim` (`self.ButtonMesh1`) (`self.Interaction1`) ByTracker))

(event `self.Interaction1.OnInteractBegin`
  (params (ByTracker :type "InteractionTrackerComponent Object Reference"))
  (`self.PressButtonAnim` (`self.ButtonMesh2`) (`self.Interaction2`) ByTracker))

(event `self.Interaction3.OnInteractBegin`
  (params (ByTracker :type "InteractionTrackerComponent Object Reference"))
  (`self.PressButtonAnim` (`self.ButtonMesh3`) (`self.Interaction3`) ByTracker))

(event `self.InteractionDone.OnInteractBegin`
  (params (ByTracker :type "InteractionTrackerComponent Object Reference"))
  (`self.PressButtonAnim` (`self.ButtonMeshDone`) (`self.InteractionDone`) ByTracker))

(fn `UserConstructionScript`
  (`parent.UserConstructionScript`))
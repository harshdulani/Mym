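; Base Blueprint for prop machines with three labelled interactions plus a Done interaction, caching the shop game state on BeginPlay.
; The construction script copies each text component's text into the matching interaction's prompt string.
; PressButtonAnim slides a given button mesh along its local Y through one shared timeline, so overlapping presses break each other's animation.
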(event `PressButtonAnim`
  (params (Mesh :type "StaticMeshComponent Object Reference") (Interaction :type "InteractionComponent Object Reference") (InteractionTracker :type "InteractionTrackerComponent Object Reference"))
  ; this timeline is a single instance, so it will break animations for other buttons if called in the middle of another button's anim
  (bind (_direction _localy) (`Timeline|Timeline` :!via `PlayFromStart`)
    (:`Update`
      (`SceneComponent.K2_SetRelativeLocation` Mesh (`KismetMathLibrary.MakeVector` 0.0 (* _localy -5.0)) false false))))

(event `self.ReceiveBeginPlay`
  ; Check construction script for text values being set
  (`parent.ReceiveBeginPlay`)
  (bind _asgs_shop_state (cast `/Game/_Game/Core/GS_ShopState` (`GameplayStatics.GetGameState`)))
  (set `self.Shop State` _asgs_shop_state))

(fn `UserConstructionScript`
  (`parent.UserConstructionScript`)
  (`|ExecutionSequence`
    (:`then_0`
      (set `InteractionComponent.InteractionString` (`KismetTextLibrary.Conv_TextToString` (`TextRenderComponent.Text` (`self.Text1`))) (`self.Interaction1`)))
    (:`then_1`
      (set `InteractionComponent.InteractionString` (`KismetTextLibrary.Conv_TextToString` (`TextRenderComponent.Text` (`self.Text2`))) (`self.Interaction2`)))
    (:`then_2`
      (set `InteractionComponent.InteractionString` (`KismetTextLibrary.Conv_TextToString` (`TextRenderComponent.Text` (`self.Text3`))) (`self.Interaction3`)))
    (:`then_3`
      (set `InteractionComponent.InteractionString` (`KismetTextLibrary.Conv_TextToString` (`TextRenderComponent.Text` (`self.TextDone`))) (`self.InteractionDone`)))))
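; A vending machine prop that lets players buy wood or blue, white and yellow paint through four interactable buttons.
; Each interaction animates its button, then calls the interacting character's Shopper to attempt an authority-side purchase at the machine's resource spawn point.
; Purchase logic lives in the Shopper, so the machine only maps buttons to products.
; Despite its name, the "Done" button purchases yellow paint.
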(event `self.Interaction1.OnInteractBegin`
  (params (ByTracker :type "InteractionTrackerComponent Object Reference"))
  (bind _mymcharacter (`InteractionTrackerComponent.MymCharacter` ByTracker))
  (`self.PressButtonAnim` (`self.ButtonMesh1`) (`self.Interaction1`) ByTracker)
  (`ShopperComponent.TryPurchaseWood_Auth` (`MymCharacter.Shopper` _mymcharacter) (`MymCharacter.GetMymPC` _mymcharacter) (`SceneComponent.K2_GetComponentToWorld` (`self.ResourceSpawnPoint`))))

(event `self.Interaction2.OnInteractBegin`
  (params (ByTracker :type "InteractionTrackerComponent Object Reference"))
  (bind _mymcharacter (`InteractionTrackerComponent.MymCharacter` ByTracker))
  (`self.PressButtonAnim` (`self.ButtonMesh2`) (`self.Interaction2`) ByTracker)
  (`ShopperComponent.TryPurchasePaint_Auth` (`MymCharacter.Shopper` _mymcharacter) (`MymCharacter.GetMymPC` _mymcharacter) "ECO_Blue" (`SceneComponent.K2_GetComponentToWorld` (`self.ResourceSpawnPoint`))))

(event `self.Interaction3.OnInteractBegin`
  (params (ByTracker :type "InteractionTrackerComponent Object Reference"))
  (bind _mymcharacter (`InteractionTrackerComponent.MymCharacter` ByTracker))
  (`self.PressButtonAnim` (`self.ButtonMesh3`) (`self.Interaction3`) ByTracker)
  (`ShopperComponent.TryPurchasePaint_Auth` (`MymCharacter.Shopper` _mymcharacter) (`MymCharacter.GetMymPC` _mymcharacter) "ECO_White" (`SceneComponent.K2_GetComponentToWorld` (`self.ResourceSpawnPoint`))))

(event `self.InteractionDone.OnInteractBegin`
  (params (ByTracker :type "InteractionTrackerComponent Object Reference"))
  (bind _mymcharacter (`InteractionTrackerComponent.MymCharacter` ByTracker))
  (`self.PressButtonAnim` (`self.ButtonMeshDone`) (`self.InteractionDone`) ByTracker)
  (`ShopperComponent.TryPurchasePaint_Auth` (`MymCharacter.Shopper` _mymcharacter) (`MymCharacter.GetMymPC` _mymcharacter) "ECO_Yellow" (`SceneComponent.K2_GetComponentToWorld` (`self.ResourceSpawnPoint`))))

(fn `UserConstructionScript`)
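; BP_MachineBase is a machine prop with three numbered interaction buttons and a Done button.
; Construction copies each button's text into its interaction prompt, and BeginPlay caches GS_ShopState.
; Each press nudges the button mesh through one shared timeline, so overlapping presses break the animation.
; Only button 1 does more, asking the player's Shopper to buy BP_Wood at the resource spawn point.
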(event `PressButtonAnim`
  (params (Mesh :type "StaticMeshComponent Object Reference") (Interaction :type "InteractionComponent Object Reference") (InteractionTracker :type "InteractionTrackerComponent Object Reference"))
  ; this is a single instance, so it will break animations for other buttons if called in the middle of another button's anim
  (bind (_direction _localy) (`Timeline|Timeline` :!via `PlayFromStart`)
    (:`Update`
      (`SceneComponent.K2_SetRelativeLocation` Mesh (`KismetMathLibrary.MakeVector` 0.0 (* _localy -5.0)) false false))))

(event `self.ReceiveBeginPlay`
  ; Check construction script for text values being set
  (`parent.ReceiveBeginPlay`)
  (bind _asgs_shop_state (cast `/Game/_Game/Core/GS_ShopState` (`GameplayStatics.GetGameState`)))
  (set `self.Shop State` _asgs_shop_state))

(event `self.OnInteract1Begin_Event`
  (params (ByTracker :type "InteractionTrackerComponent Object Reference"))
  (bind _mymcharacter (`InteractionTrackerComponent.MymCharacter` ByTracker))
  (`self.PressButtonAnim` (`self.ButtonMesh1`) (`self.Interaction1`) ByTracker)
  (`ShopperComponent.TryPurchase_Auth` (`MymCharacter.Shopper` _mymcharacter) (`MymCharacter.GetMymPC` _mymcharacter) 50 "/Game/_Game/Props/Resources/BP_Wood.BP_Wood_C" (`SceneComponent.K2_GetComponentToWorld` (`self.ResourceSpawnPoint`))))

(event `self.OnInteract2Begin_Event`
  (params (ByTracker :type "InteractionTrackerComponent Object Reference"))
  (`self.PressButtonAnim` (`self.ButtonMesh2`) (`self.Interaction2`) ByTracker))

(event `self.OnInteract3Begin_Event`
  (params (ByTracker :type "InteractionTrackerComponent Object Reference"))
  (`self.PressButtonAnim` (`self.ButtonMesh3`) (`self.Interaction3`) ByTracker))

(event `self.OnInteractDoneBegin_Event`
  (params (ByTracker :type "InteractionTrackerComponent Object Reference"))
  (`self.PressButtonAnim` (`self.ButtonMeshDone`) (`self.InteractionDone`) ByTracker))

(fn `UserConstructionScript`
  (`parent.UserConstructionScript`)
  (`|ExecutionSequence`
    (:`then_0`
      (set `InteractionComponent.InteractionString` (`KismetTextLibrary.Conv_TextToString` (`TextRenderComponent.Text` (`self.Text1`))) (`self.Interaction1`)))
    (:`then_1`
      (set `InteractionComponent.InteractionString` (`KismetTextLibrary.Conv_TextToString` (`TextRenderComponent.Text` (`self.Text2`))) (`self.Interaction2`)))
    (:`then_2`
      (set `InteractionComponent.InteractionString` (`KismetTextLibrary.Conv_TextToString` (`TextRenderComponent.Text` (`self.Text3`))) (`self.Interaction3`)))
    (:`then_3`
      (set `InteractionComponent.InteractionString` (`KismetTextLibrary.Conv_TextToString` (`TextRenderComponent.Text` (`self.TextDone`))) (`self.InteractionDone`)))))